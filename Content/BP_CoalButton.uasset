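; BP_CoalButton is a clickable coal actor that acts as the main click-to-earn button in a pollution-themed game.
; Clicking its visual adds the click value to the coal total in BP_PollutionGameInstance and prints the total.
; A counter there triggers SpawnFactory on the game instance and resets once it reaches a coal threshold.
; Each click also plays a timeline scale animation on the visual and a ping sound.
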(event OnClicked(CoalVisual)
  (params (TouchedComponent :type Primitive%20Component%20Object%20Reference) (ButtonPressed :type Key%20Structure :default "None"))
  (Utilities|FlowControl|Sequence
    (:then_0
      (bind _asbp_pollution_game_instance (Utilities|Casting|CastToBP_PollutionGameInstance (Game|GetGameInstance)))
      ;[0.15 0.15 0.15 0.5] Update Coal +1
      (bind _output_get (Variables|/Game/BP_PollutionGameInstance.BP_PollutionGameInstance_C|SetTotalCoal _asbp_pollution_game_instance (Math|Float|Truncate (+ (Variables|/Game/BP_PollutionGameInstance.BP_PollutionGameInstance_C|GetTotalCoal _asbp_pollution_game_instance) (Variables|/Game/BP_PollutionGameInstance.BP_PollutionGameInstance_C|GetClickValue _asbp_pollution_game_instance)))))
      (Development|PrintString (Utilities|String|ToString(Integer) _output_get))
      ;[0.15 0.15 0.15 0.5] Spawn Factory every 10 coal
      (bind _output_get_2 (Variables|/Game/BP_PollutionGameInstance.BP_PollutionGameInstance_C|SetCoalSinceLastFactory _asbp_pollution_game_instance (Math|Float|Truncate (+ (Variables|/Game/BP_PollutionGameInstance.BP_PollutionGameInstance_C|GetClickValue _asbp_pollution_game_instance) (Variables|/Game/BP_PollutionGameInstance.BP_PollutionGameInstance_C|GetCoalSinceLastFactory _asbp_pollution_game_instance)))))
      (if (>= _output_get_2 10)
        (Default|SpawnFactory _asbp_pollution_game_instance)
        (Variables|/Game/BP_PollutionGameInstance.BP_PollutionGameInstance_C|SetCoalSinceLastFactory _asbp_pollution_game_instance 0)))
    (:then_1
      ;[0.15 0.15 0.15 0.5] Animation and Sound
      (bind _scale (Timeline|TL_ClickScale PlayFromStart)
        (:Update
          (Transformation|SetRelativeScale3D (Variables|Default|GetCoalVisual) (Math|Vector|MakeVector _scale _scale _scale)))))
    (:then_2
      (Audio|PlaySoundatLocation "/Engine/EngineSounds/1kSineTonePing.1kSineTonePing" "0, 0, 0" "0, 0, 0" 1.0 1.0 0.0 0 0 0 0))))

(event EventBeginPlay)

(event Collision|EventActorBeginOverlap
  (params (OtherActor :type Actor%20Object%20Reference)))

(event EventTick
  (params (DeltaSeconds :type Float%20%28single-precision%29)))

(fn ConstructionScript)