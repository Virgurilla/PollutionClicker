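; Clickable actor for a clicker game that earns crypto each time its CoalVisual component is clicked.
; A click adds the game instance's ClickValue to both the crypto total and a counter since the last factory.
; When that counter reaches the threshold, it calls SpawnFactory on the game instance, resets the counter to zero and plays a drop sound.
; Every click also runs a timeline scale animation on the visual and plays a ping.
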(event OnClicked(CoalVisual)
  (params (TouchedComponent :type Primitive%20Component%20Object%20Reference) (ButtonPressed :type Key%20Structure :default "None"))
  (bind _result (CallFunction|GetPollutionGameInstance))
  (bind _clickvalue (Variables|/Game/BP_PollutionGameInstance.BP_PollutionGameInstance_C|GetClickValue _result))
  (Utilities|FlowControl|Sequence
    (:then_0
      ;[0.15 0.15 0.15 0.5] Update Coal +1
      (Variables|/Game/BP_PollutionGameInstance.BP_PollutionGameInstance_C|SetTotalCrypto _result (Math|Float|Truncate (+ (Variables|/Game/BP_PollutionGameInstance.BP_PollutionGameInstance_C|GetTotalCrypto _result) _clickvalue)))
      ;[0.15 0.15 0.15 0.5] Spawn Factory every 10 coal
      (bind _output_get (Variables|/Game/BP_PollutionGameInstance.BP_PollutionGameInstance_C|SetCryptoSinceLastFactory _result (Math|Float|Truncate (+ _clickvalue (Variables|/Game/BP_PollutionGameInstance.BP_PollutionGameInstance_C|GetCryptoSinceLastFactory _result)))))
      (if (>= _output_get 10)
        (Default|SpawnFactory _result)
        (Variables|/Game/BP_PollutionGameInstance.BP_PollutionGameInstance_C|SetCryptoSinceLastFactory _result 0)
        (Audio|PlaySoundatLocation "/Engine/VREditor/Sounds/UI/Dockable_Window_Drop.Dockable_Window_Drop" "0, 0, 0" "0, 0, 0" 1.0 1.0 0.0 0 0 0 0)))
    (:then_1
      ;[0.15 0.15 0.15 0.5] Animation and Sound
      (bind _scale (Timeline|TL_ClickScale PlayFromStart)
        (:Update
          (Transformation|SetRelativeScale3D (Variables|Default|GetCoalVisual) (Math|Vector|MakeVector _scale _scale _scale)))))
    (:then_2
      (Audio|PlaySoundatLocation "/Engine/EngineSounds/1kSineTonePing.1kSineTonePing" "0, 0, 0" "0, 0, 0" 1.0 1.0 0.0 0 0 0 0))))

(event EventBeginPlay)

(event Collision|EventActorBeginOverlap
  (params (OtherActor :type Actor%20Object%20Reference)))

(event EventTick
  (params (DeltaSeconds :type Float%20%28single-precision%29)))

(fn ConstructionScript)