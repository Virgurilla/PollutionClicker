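; BP_Factory is a placed factory that passively produces coal in the pollution game.
; A looping timer set from the game instance's production rate calls ProduceCoal, which raises the instance's TotalCoal and FactoryCoal and plays a sound and smoke effect.
; Each tick also advances CoalSinceLastFactory by ClickValue rather than the factory's production value, asking the game instance to spawn another factory and resetting at a ten-coal threshold.
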(event EventBeginPlay
  (bind _asbp_pollution_game_instance (Utilities|Casting|CastToBP_PollutionGameInstance (Game|GetGameInstance)))
  (Utilities|Time|SetTimerbyFunctionName 0 "ProduceCoal" (Variables|/Game/BP_PollutionGameInstance.BP_PollutionGameInstance_C|GetFactoryProductionRate _asbp_pollution_game_instance) true))

(fn ConstructionScript)

(fn ProduceCoal
  (bind _result (CallFunction|GetPollutionGameInstance))
  (bind _factoryproductionvalue (Variables|/Game/BP_PollutionGameInstance.BP_PollutionGameInstance_C|GetFactoryProductionValue _result))
  ;[0.15 0.15 0.15 0.5] Increase TotalCoal
  (bind _output_get (Variables|/Game/BP_PollutionGameInstance.BP_PollutionGameInstance_C|SetTotalCoal _result (Math|Float|Truncate (+ (Variables|/Game/BP_PollutionGameInstance.BP_PollutionGameInstance_C|GetTotalCoal _result) _factoryproductionvalue))))
  (Development|PrintString (Utilities|String|ToString(Integer) _output_get))
  (Utilities|FlowControl|Sequence
    (:then_0
      ;[0.15 0.15 0.15 0.5] Spawn Factory every 10 coal
      (bind _output_get_2 (Variables|/Game/BP_PollutionGameInstance.BP_PollutionGameInstance_C|SetCoalSinceLastFactory _result (Math|Float|Truncate (+ (Variables|/Game/BP_PollutionGameInstance.BP_PollutionGameInstance_C|GetClickValue _result) (Variables|/Game/BP_PollutionGameInstance.BP_PollutionGameInstance_C|GetCoalSinceLastFactory _result)))))
      (if (>= _output_get_2 10)
        (Default|SpawnFactory _result)
        (Variables|/Game/BP_PollutionGameInstance.BP_PollutionGameInstance_C|SetCoalSinceLastFactory _result 0)))
    (:then_1
      ;[0.15 0.15 0.15 0.5] IncreaseFactoryCoal
      (Variables|/Game/BP_PollutionGameInstance.BP_PollutionGameInstance_C|SetFactoryCoal _result (Math|Float|Truncate (+ _factoryproductionvalue (Variables|/Game/BP_PollutionGameInstance.BP_PollutionGameInstance_C|GetFactoryCoal _result))))
      ;[0.15 0.15 0.15 0.5] Factory production Sound and Particle
      (Audio|PlaySoundatLocation "/Engine/VREditor/Sounds/UI/Floating_UI_Open-001.Floating_UI_Open-001" (Transformation|GetActorLocation) "0, 0, 0" 1.0 1.0 0.0 0 0 0 0)
      (Niagara|SpawnSystematLocation "/Game/NS_FactorySmoke.NS_FactorySmoke" (Transformation|GetWorldLocation (Variables|Default|GetSmokeSpawnPoint))))))