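; Game instance for a pollution clicker game, holding the crypto economy, factory spawning, upgrades and win condition.
; Three two-level upgrade tracks spend crypto to improve click value, factory rate and factory value, with rate upgrades resetting every factory's timer.
; Factories spawn at random points within the bounds of the first StaticMeshActor found.
; Reaching the pollution goal shows the win widget with UI-only input and stops all factory production.
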(fn SpawnFactory
  (bind _returnvalue (Actor|GetActorOfClass "/Script/Engine.StaticMeshActor"))
  (Game|SpawnActorfromClass "/Game/BP_Factory.BP_Factory_C" (Math|Conversions|ToTransform(Vector) (Math|Vector|MakeVector (.X (Math|Vector|BreakVector (Math|Random|RandomPointinBoundingBox (.Origin (Collision|GetActorBounds _returnvalue false false)) (.BoxExtent (Collision|GetActorBounds _returnvalue false false))))) (.Y (Math|Vector|BreakVector (Math|Random|RandomPointinBoundingBox (.Origin (Collision|GetActorBounds _returnvalue false false)) (.BoxExtent (Collision|GetActorBounds _returnvalue false false))))) (+ (+ (.Z (Math|Vector|BreakVector (Math|Random|RandomPointinBoundingBox (.Origin (Collision|GetActorBounds _returnvalue false false)) (.BoxExtent (Collision|GetActorBounds _returnvalue false false))))) 2.0) (Math|Random|RandomFloat)))) "Undefined" "MultiplyWithRoot" 0 0))

(fn UpgradeClick
  (if (>= (Variables|Default|GetUpgrade_ClickLevel) 2)
    (return false)
    (else
      (bind _output_get (Variables|Default|SetUpgradeCost (Utilities|Array|Get(acopy) (Variables|Default|GetUpgrade_ClickCosts) (Variables|Default|GetUpgrade_ClickLevel))))
      (if (> (Variables|Default|GetTotalCrypto) _output_get)
        (Variables|Default|SetTotalCrypto (- (Variables|Default|GetTotalCrypto) _output_get))
        (bind _output_get_2 (Variables|Default|SetUpgrade_ClickLevel (+ (Variables|Default|GetUpgrade_ClickLevel) 1)))
        (switch int _output_get_2
          (:1
            (Variables|Default|SetClickValue 2.0)
            (return true))
          (:2
            (Variables|Default|SetClickValue 3.0)
            (return true)))
        (else
          (return false))))))

(fn UpgradeFactoryRate
  (if (>= (Variables|Default|GetUpgrade_FactoryRateLevel) 2)
    (return false)
    (else
      (bind _output_get (Variables|Default|SetUpgradeCost (Utilities|Array|Get(acopy) (Variables|Default|GetUpgrade_RateCosts) (Variables|Default|GetUpgrade_FactoryRateLevel))))
      (if (> (Variables|Default|GetTotalCrypto) _output_get)
        (Variables|Default|SetTotalCrypto (- (Variables|Default|GetTotalCrypto) _output_get))
        (bind _output_get_2 (Variables|Default|SetUpgrade_FactoryRateLevel (+ (Variables|Default|GetUpgrade_FactoryRateLevel) 1)))
        (switch int _output_get_2
          (:1
            (Variables|Default|SetFactoryProductionRate 2.0))
          (:2
            (Variables|Default|SetFactoryProductionRate 1.0)))
        (bind _outactors (Actor|GetAllActorsOfClass "/Game/BP_Factory.BP_Factory_C"))
        (for _array_element _outactors
          (Default|ResetProductionTimer _array_element))
        (return true)
        (else
          (return false))))))

(fn UpgradeFactoryValue
  (if (>= (Variables|Default|GetUpgrade_FactoryValueLevel) 2)
    (return false)
    (else
      (bind _output_get (Variables|Default|SetUpgradeCost (Utilities|Array|Get(acopy) (Variables|Default|GetUpgrade_ValueCosts) (Variables|Default|GetUpgrade_FactoryValueLevel))))
      (if (> (Variables|Default|GetTotalCrypto) _output_get)
        (Variables|Default|SetTotalCrypto (- (Variables|Default|GetTotalCrypto) _output_get))
        (bind _output_get_2 (Variables|Default|SetUpgrade_FactoryValueLevel (+ (Variables|Default|GetUpgrade_FactoryValueLevel) 1)))
        (switch int _output_get_2
          (:1
            (Variables|Default|SetFactoryProductionValue 1.5)
            (return true))
          (:2
            (Variables|Default|SetFactoryProductionValue 2.0)
            (return true)))
        (else
          (return false))))))

(fn CheckWinCondition
  (if (>= (Variables|Default|GetGeneratedPollution) (Variables|Default|GetPollutionGoal))
    (CallFunction|TriggerWin)))

(fn TriggerWin
  (Utilities|FlowControl|Sequence
    (:then_0
      (bind _returnvalue (Class|InputDeviceLibrary|GetPlayerControllerfromPlatformUser))
      (bind _returnvalue_2 (UserInterface|CreateWidget "/Game/WBP_YouWin.WBP_YouWin_C" _returnvalue))
      (UserInterface|Viewport|AddtoViewport _returnvalue_2 0)
      (Input|SetInputModeUIOnly _returnvalue _returnvalue_2 "DoNotLock" false)
      (Variables|/Script/Engine.PlayerController|SetbShowMouseCursor _returnvalue true))
    (:then_1
      (bind _outactors (Actor|GetAllActorsOfClass "/Game/BP_Factory.BP_Factory_C"))
      (for _array_element _outactors
        (Default|StopProduction _array_element)))))