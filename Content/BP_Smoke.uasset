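; BP_Smoke drives a smoke material on its owner's static mesh to reflect the game's pollution progress.
; On BeginPlay it creates a dynamic instance of M_Smoke and assigns it to the first material slot of that mesh.
; Every Tick it sets the SmokeIntensity parameter to generated pollution divided by the pollution goal, both read from the pollution game instance and clamped between zero and one.
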(event EventBeginPlay
  (bind _returnvalue (Rendering|Material|CreateDynamicMaterialInstance "/Game/Sprites/M_Smoke.M_Smoke" "None" "None" :!class /Script/Engine.KismetMaterialLibrary))
  (bind _output_get (Variables|Default|SetNewVar _returnvalue))
  (Rendering|Material|SetMaterial (Actor|GetComponentbyClass (Components|GetOwner) "/Script/Engine.StaticMeshComponent") 0 _output_get))

(event EventTick
  (params (DeltaSeconds :type Float%20%28single-precision%29))
  (bind _result (CallFunction|GetPollutionGameInstance))
  (Rendering|Material|SetScalarParameterValue (stale EventBeginPlay _output_get) "SmokeIntensity" (Math|Float|Clamp(Float) (/ (Math|Conversions|ToFloat(Integer) (Variables|/Game/BP_PollutionGameInstance.BP_PollutionGameInstance_C|GetGeneratedPollution _result)) (Variables|/Game/BP_PollutionGameInstance.BP_PollutionGameInstance_C|GetPollutionGoal _result))) :!class /Script/Engine.MaterialInstanceDynamic))